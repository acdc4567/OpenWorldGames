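; Shooter HUD that draws a dynamic green crosshair at screen center, made of a center dot and four directional pieces.
; BeginPlay caches the player's BP_ShooterCharacter, and Tick polls its crosshair spread multiplier.
; DrawHUD offsets the left, right, top and bottom textures outward by that multiplier times a maximum spread, while the dot stays fixed.
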(event EventBeginPlay
  (bind _asbp_shooter_character (Utilities|Casting|CastToBP_ShooterCharacter (Game|Player|GetPlayerPawn 0)))
  (Variables|Default|SetAs%20BP%20Shooter%20Character _asbp_shooter_character))

(event Collision|EventActorBeginOverlap
  (params (OtherActor :type Actor%20Object%20Reference)))

(event EventTick
  (params (DeltaSeconds :type Float%20%28single-precision%29))
  (Variables|Default|SetSpreadMUltiplier (Class|ShooterCharacter|GetCrosshairSpreadMultiplier (Variables|Default|GetAs%20BP%20Shooter%20Character))))

(event EventDrawHUD
  (params (SizeX :type Integer) (SizeY :type Integer))
  (Variables|Default|SetScreenCenter (Math|Vector2D|MakeVector2D (Math|Conversions|ToFloat(Integer) (/ SizeX 2)) (Math|Conversions|ToFloat(Integer) (/ SizeY 2))))
  (Canvas|DrawTexture "/Game/Sounds/Icons/Crosshairs_Edited/Crosshair_Dot.Crosshair_Dot" (- (.X (Math|Vector2D|BreakVector2D (Variables|Default|GetScreenCenter))) (Variables|Default|GetCrossXOffset)) (- (.Y (Math|Vector2D|BreakVector2D (Variables|Default|GetScreenCenter))) (Variables|Default|GetCrossYOffset)) 64.0 64.0 0.0 0.0 1.0 1.0 "(R=0.049283,G=1.000000,B=0.088440,A=1.000000)")
  (Canvas|DrawTexture "/Game/Sounds/Icons/Crosshairs_Edited/Crosshair_Quad_9_Right.Crosshair_Quad_9_Right" (+ (- (.X (Math|Vector2D|BreakVector2D (Variables|Default|GetScreenCenter))) (Variables|Default|GetCrossXOffset)) (* (Variables|Default|GetSpreadMUltiplier) (Variables|Default|GetCrosshairSpreadMax))) (- (.Y (Math|Vector2D|BreakVector2D (Variables|Default|GetScreenCenter))) (Variables|Default|GetCrossYOffset)) 64.0 64.0 0.0 0.0 1.0 1.0 "(R=0.049283,G=1.000000,B=0.088440,A=1.000000)")
  (Canvas|DrawTexture "/Game/Sounds/Icons/Crosshairs_Edited/Crosshair_Quad_9_Left.Crosshair_Quad_9_Left" (- (- (.X (Math|Vector2D|BreakVector2D (Variables|Default|GetScreenCenter))) (Variables|Default|GetCrossXOffset)) (* (Variables|Default|GetSpreadMUltiplier) (Variables|Default|GetCrosshairSpreadMax))) (- (.Y (Math|Vector2D|BreakVector2D (Variables|Default|GetScreenCenter))) (Variables|Default|GetCrossYOffset)) 64.0 64.0 0.0 0.0 1.0 1.0 "(R=0.049283,G=1.000000,B=0.088440,A=1.000000)")
  (Canvas|DrawTexture "/Game/Sounds/Icons/Crosshairs_Edited/Crosshair_Quad_9_Top.Crosshair_Quad_9_Top" (- (.X (Math|Vector2D|BreakVector2D (Variables|Default|GetScreenCenter))) (Variables|Default|GetCrossXOffset)) (- (- (.Y (Math|Vector2D|BreakVector2D (Variables|Default|GetScreenCenter))) (Variables|Default|GetCrossYOffset)) (* (Variables|Default|GetSpreadMUltiplier) (Variables|Default|GetCrosshairSpreadMax))) 64.0 64.0 0.0 0.0 1.0 1.0 "(R=0.049283,G=1.000000,B=0.088440,A=1.000000)")
  (Canvas|DrawTexture "/Game/Sounds/Icons/Crosshairs_Edited/Crosshair_Quad_9_Bottom.Crosshair_Quad_9_Bottom" (- (.X (Math|Vector2D|BreakVector2D (Variables|Default|GetScreenCenter))) (Variables|Default|GetCrossXOffset)) (+ (- (.Y (Math|Vector2D|BreakVector2D (Variables|Default|GetScreenCenter))) (Variables|Default|GetCrossYOffset)) (* (Variables|Default|GetSpreadMUltiplier) (Variables|Default|GetCrosshairSpreadMax))) 64.0 64.0 0.0 0.0 1.0 1.0 "(R=0.049283,G=1.000000,B=0.088440,A=1.000000)"))

(fn ConstructionScript)