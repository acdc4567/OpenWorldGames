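; BP_Enemy2 is an enemy Blueprint that carries a health bar widget on a HealthBar component.
; On BeginPlay it passes itself to the WBP_EnemyHealthBar widget as EnemyRef and hides the bar.
; Show and hide events toggle the widget's visibility, with the show event also calling its parent implementation.
; The hit number event is overridden with no logic.
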(event EventBeginPlay
  (bind _aswbp_enemy_health_bar (Utilities|Casting|CastToWBP_EnemyHealthBar (UserInterface|GetUserWidgetObject (Variables|Default|GetHealthBar))))
  (Variables|/Game/_Game/HUD/WBP_EnemyHealthBar.WBP_EnemyHealthBar_C|SetEnemyRef _aswbp_enemy_health_bar self)
  (Widget|SetVisibility (UserInterface|GetUserWidgetObject (Variables|Default|GetHealthBar)) "Hidden"))

(event Collision|EventActorBeginOverlap
  (params (OtherActor :type Actor%20Object%20Reference)))

(event EventTick
  (params (DeltaSeconds :type Float%20%28single-precision%29)))

(event EventShowHealthBar
  (Widget|SetVisibility (UserInterface|GetUserWidgetObject (Variables|Default|GetHealthBar)) "Visible")
  (|CallParentFunction))

(event EventHideHealthBar
  (Widget|SetVisibility (UserInterface|GetUserWidgetObject (Variables|Default|GetHealthBar)) "Hidden"))

(event EventShowHitNumber
  (params (Damage :type Integer) (HitLocation :type Vector :default "0, 0, 0")))

(fn ConstructionScript)