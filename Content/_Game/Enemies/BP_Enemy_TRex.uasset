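; T-Rex enemy Blueprint that manages the health bar widget for this enemy type.
; On BeginPlay it casts its widget component's user widget to the T-Rex health bar, passes itself as a reference and hides the bar.
; ShowHealthBar reveals the widget then calls the parent version, while HideHealthBar hides it without a parent call.
; ShowHitNumber is left empty.
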(event EventBeginPlay
  (bind _aswbp_enemy_health_bar_trex (Utilities|Casting|CastToWBP_EnemyHealthBar_Trex (UserInterface|GetUserWidgetObject (Variables|Default|GetWidget))))
  (Variables|/Game/_Game/HUD/WBP_EnemyHealthBar_Trex.WBP_EnemyHealthBar_Trex_C|SetTrexEnemyRef _aswbp_enemy_health_bar_trex self)
  (Widget|SetVisibility (UserInterface|GetUserWidgetObject (Variables|Default|GetWidget)) "Hidden"))

(event Collision|EventActorBeginOverlap
  (params (OtherActor :type Actor%20Object%20Reference)))

(event EventTick
  (params (DeltaSeconds :type Float%20%28single-precision%29)))

(event EventShowHealthBar
  (Widget|SetVisibility (UserInterface|GetUserWidgetObject (Variables|Default|GetWidget)) "Visible")
  (|CallParentFunction))

(event EventHideHealthBar
  (Widget|SetVisibility (UserInterface|GetUserWidgetObject (Variables|Default|GetWidget)) "Hidden"))

(event EventShowHitNumber
  (params (Damage :type Integer) (HitLocation :type Vector :default "0, 0, 0")))

(fn ConstructionScript)