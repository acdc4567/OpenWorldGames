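; BP_MixConrvCharx is a human knight character Blueprint that handles player input for camera look and an evade animation.
; Mouse axes feed controller yaw and pitch directly.
; Movement axes are lerp-smoothed into Speed and Direction variables, with no movement input applied in this graph.
; NumPad One plays an aerial evade montage on the mesh through a hard-wired key event.
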(event EventBeginPlay)

(event Collision|EventActorBeginOverlap
  (params (OtherActor :type Actor%20Object%20Reference)))

(event EventTick
  (params (DeltaSeconds :type Float%20%28single-precision%29)))

(event Input|AxisEvents|InputAxisTurnRight/LeftMouse
  (params (AxisValue :type Float%20%28single-precision%29))
  (Pawn|Input|AddControllerYawInput AxisValue))

(event Input|AxisEvents|InputAxisLookUp/DownMouse
  (params (AxisValue :type Float%20%28single-precision%29))
  (Pawn|Input|AddControllerPitchInput AxisValue))

(event Input|AxisEvents|InputAxisMoveForward/Backward
  (params (AxisValue :type Float%20%28single-precision%29))
  (bind _output_get (Variables|Default|SetSpeed (Math|Float|Lerp (stale _output_get) AxisValue 0.05))))

(event Input|AxisEvents|InputAxisMoveRight/Left
  (params (AxisValue :type Float%20%28single-precision%29))
  (bind _output_get (Variables|Default|SetDirection (Math|Float|Lerp (stale _output_get) AxisValue 0.05))))

(event Input|KeyboardEvents|NumPadOne
  (params (Key :type Key%20Structure :default "None"))
  (:Pressed
    (Animation|Montage|PlayMontage (Variables|Character|GetMesh) "/Game/KnightCharacter/MannyAnims/AerialEvade4UE4_Montage.AerialEvade4UE4_Montage")))

(fn ConstructionScript)