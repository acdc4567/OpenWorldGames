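; BP_Playerx is a human knight player character that supports upper-body aiming with a bow.
; Each tick, UpperBodyRotatun stores control pitch and yaw and, without a bow, zeroes ModifyBoneAlpha.
; With a bow, it sets that alpha to 1 within a yaw threshold, otherwise interpolates the actor toward control yaw.
; NumPad 2 swaps the mesh's animation Blueprint while held; older AnimBP message calls are left disconnected.
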(event EventBeginPlay
  (|CallParentFunction) ; This node is disabled and will not be called.\nDrag off pins to build functionality.
)

(event Collision|EventActorBeginOverlap
  (params (OtherActor :type Actor%20Object%20Reference))
  (|CallParentFunction OtherActor) ; This node is disabled and will not be called.\nDrag off pins to build functionality.
)

(event EventTick
  (params (DeltaSeconds :type Float%20%28single-precision%29))
  (|CallParentFunction DeltaSeconds)
  (|UpperBodyRotatun DeltaSeconds))

(event Input|KeyboardEvents|NumPadTwo
  (params (Key :type Key%20Structure :default "None"))
  (:Pressed
    (Class|SkeletalMeshComponent|SetAnimClass (Variables|Character|GetMesh) "/Game/KnightCharacter/Human/ABP_Human1.ABP_Human1_C"))
  (:Released
    (Class|SkeletalMeshComponent|SetAnimClass (Variables|Character|GetMesh) "/Game/KnightCharacter/Human/ABP_Human.ABP_Human_C")))

(fn ConstructionScript
  (|CallParentFunction))