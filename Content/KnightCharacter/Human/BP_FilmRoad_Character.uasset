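; BP_FilmRoad_Character is a player-controlled human character with camera-relative movement, mouse look and a sprint flag on Left Shift.
; Axis events store inputs; strafing applies there, while forward movement applies on Tick, both along control yaw.
; Tick also derives a Direction angle from follow camera, capsule and input rotations, printing it alongside axis values for debugging.
; NumPad 1 plays a 90-degree turn montage, apparently as a test.
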(event EventBeginPlay)

(event Collision|EventActorBeginOverlap
  (params (OtherActor :type Actor%20Object%20Reference)))

(event EventTick
  (params (DeltaSeconds :type Float%20%28single-precision%29))
  (Utilities|FlowControl|Sequence
    (:then_0
      (bind _output_get (Variables|Default|SetDirection (.yaw (Math|Rotator|Delta(Rotator) (Math|Rotator|Delta(Rotator) (Transformation|GetWorldRotation (Variables|Default|GetFollowCamera)) (Transformation|GetWorldRotation (Variables|Collision|GetCapsuleComponent))) (Math|Conversions|RotationFromXVector (Math|Vector|MakeVector (stale Input|AxisEvents|InputAxisMoveForward/Backward AxisValue) (* (stale Input|AxisEvents|InputAxisMoveRight/Left AxisValue) -1.0) 0.0))))))
      (Development|PrintString (Utilities|String|Append "Direction :" (Utilities|String|ToString(Float) _output_get)) true true "(R=0.000000,G=0.660000,B=1.000000,A=1.000000)" 0.0)
      (Pawn|Input|AddMovementInput (Math|Vector|GetForwardVector (Math|Rotator|MakeRotator 0.0 0.0 (.yaw (Pawn|GetControlRotation :!class /Script/Engine.Pawn)))) (Variables|Default|GetInputZ) false))))

(event Input|AxisEvents|InputAxisMoveForward/Backward
  (params (AxisValue :type Float%20%28single-precision%29))
  (bind _output_get (Variables|Default|SetInputZ AxisValue))
  (Development|PrintString (Utilities|String|Append "InputZ :" (Utilities|String|ToString(Float) _output_get)) true true "(R=0.000000,G=0.660000,B=1.000000,A=1.000000)" 0.0))

(event Input|AxisEvents|InputAxisMoveRight/Left
  (params (AxisValue :type Float%20%28single-precision%29))
  (bind _output_get (Variables|Default|SetInputX AxisValue))
  (Development|PrintString (Utilities|String|Append "InputX : " (Utilities|String|ToString(Float) _output_get)) true true "(R=0.000000,G=0.660000,B=1.000000,A=1.000000)" 0.0)
  (Pawn|Input|AddMovementInput (Math|Vector|GetRightVector (Math|Rotator|MakeRotator 0.0 0.0 (.yaw (Pawn|GetControlRotation :!class /Script/Engine.Pawn)))) (Variables|Default|GetInputX) false))

(event Input|AxisEvents|InputAxisTurnRight/LeftMouse
  (params (AxisValue :type Float%20%28single-precision%29))
  (Pawn|Input|AddControllerYawInput AxisValue))

(event Input|AxisEvents|InputAxisLookUp/DownMouse
  (params (AxisValue :type Float%20%28single-precision%29))
  (Pawn|Input|AddControllerPitchInput AxisValue))

(event Input|KeyboardEvents|LeftShift
  (params (Key :type Key%20Structure :default "None"))
  (:Pressed
    (Variables|Default|SetIsSprinting true))
  (:Released
    (Variables|Default|SetIsSprinting false)))

(event Input|KeyboardEvents|NumPadOne
  (params (Key :type Key%20Structure :default "None"))
  (:Pressed
    (Animation|Montage|PlayMontage (Variables|Character|GetMesh) "/Game/KnightCharacter/MannyAnims/Manu_Turn_90_R4UE4_Montage.Manu_Turn_90_R4UE4_Montage")))

(fn ConstructionScript)