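; BP_Human is a player-controlled knight Character with basic third-person-style locomotion, jumping and footstep audio.
; Input axes drive mouse look and movement relative to control yaw, while a run toggle and held sprint set CharacterMovement's max walk speed, with sprint release always returning to running.
; Jumping plays a montage and landing replays it from its JumpLand section.
; A Footstep event plays a rock footstep sound at the actor's location.
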(event EventBeginPlay)

(event Collision|EventActorBeginOverlap
  (params (OtherActor :type Actor%20Object%20Reference)))

(event EventTick
  (params (DeltaSeconds :type Float%20%28single-precision%29)))

(event EventOnLanded
  (params (Hit :type Hit%20Result%20Structure%20%28by%20ref%29))
  (Animation|PlayAnimMontage "/Game/KnightCharacter/Knight/Anims/Knight_Run_Jump_Montage.Knight_Run_Jump_Montage" 1.0 "JumpLand"))

(event Input|ActionEvents|InputActionToggleRun
  (params (Key :type Key%20Structure :default "None"))
  (bind _charactermovement (Variables|Character|GetCharacterMovement))
  (:Pressed
    (bind _output_get (Variables|Default|SetRunning (not (Variables|Default|GetRunning))))
    (if _output_get
      (Variables|/Script/Engine.CharacterMovementComponent|SetMaxWalkSpeed _charactermovement 6e+02)
      (else
        (Variables|/Script/Engine.CharacterMovementComponent|SetMaxWalkSpeed _charactermovement 3e+02)))))

(event Input|ActionEvents|InputActionSprint
  (params (Key :type Key%20Structure :default "None"))
  (bind _charactermovement (Variables|Character|GetCharacterMovement))
  (:Pressed
    (Variables|Default|SetSprinting true)
    (Variables|/Script/Engine.CharacterMovementComponent|SetMaxWalkSpeed _charactermovement 8e+02))
  (:Released
    (Variables|Default|SetSprinting false)
    (Variables|/Script/Engine.CharacterMovementComponent|SetMaxWalkSpeed _charactermovement 6e+02)
    (Variables|Default|SetRunning true)))

(event Input|ActionEvents|InputActionJumpx
  (params (Key :type Key%20Structure :default "None"))
  (:Pressed
    (Character|Jump)
    (Animation|PlayAnimMontage "/Game/KnightCharacter/Knight/Anims/Knight_Run_Jump_Montage.Knight_Run_Jump_Montage" 1.0 "None")))

(event Input|AxisEvents|InputAxisTurnRight/LeftMouse
  (params (AxisValue :type Float%20%28single-precision%29))
  (Pawn|Input|AddControllerYawInput AxisValue))

(event Input|AxisEvents|InputAxisLookUp/DownMouse
  (params (AxisValue :type Float%20%28single-precision%29))
  (Pawn|Input|AddControllerPitchInput AxisValue))

(event Input|AxisEvents|InputAxisMoveForward/Backward
  (params (AxisValue :type Float%20%28single-precision%29))
  (Pawn|Input|AddMovementInput (Math|Vector|GetForwardVector (Math|Rotator|MakeRotator 0.0 0.0 (.Yaw (Math|Rotator|BreakRotator (Pawn|GetControlRotation :!class /Script/Engine.Pawn))))) AxisValue false))

(event Input|AxisEvents|InputAxisMoveRight/Left
  (params (AxisValue :type Float%20%28single-precision%29))
  (Pawn|Input|AddMovementInput (Math|Vector|GetRightVector (Math|Rotator|MakeRotator 0.0 0.0 (.Yaw (Math|Rotator|BreakRotator (Pawn|GetControlRotation :!class /Script/Engine.Pawn))))) AxisValue false))

(event EventFootstep
  (params (LorR :type Boolean))
  (Audio|PlaySoundatLocation "/Game/StarterContent/Footsteps/FS_Rockx1.FS_Rockx1" (Transformation|GetActorLocation) "0, 0, 0" 1.0 1.0 0.0 0 0 0 0))

(fn ConstructionScript)