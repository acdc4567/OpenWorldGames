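; BP_NPC_Enemy is an enemy human NPC in the knight character set that chases and attacks a given target.
; ToggleAttacking starts a DoOnce-guarded, Delay-driven loop, with no Tick logic.
; Within hit range it calls AIAttack at short random intervals; otherwise it periodically moves to a point just inside that range.
; The Attacking flag is rechecked only after attacks, so chasing continues when toggled off.
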(event EventBeginPlay
  (|CallParentFunction) ; This node is disabled and will not be called.\nDrag off pins to build functionality.
)

(event Collision|EventActorBeginOverlap
  (params (OtherActor :type Actor%20Object%20Reference))
  (|CallParentFunction OtherActor) ; This node is disabled and will not be called.\nDrag off pins to build functionality.
)

(event EventTick
  (params (DeltaSeconds :type Float%20%28single-precision%29))
  (|CallParentFunction DeltaSeconds) ; This node is disabled and will not be called.\nDrag off pins to build functionality.
)

(event EventToggleAttacking
  (params (Enable :type Boolean) (Enemy :type Actor%20Object%20Reference))
  (bind _returnvalue (Transformation|GetActorLocation Enemy))
  (bind _output_get (Variables|Default|SetAttacking Enable))
  (if _output_get
    (Utilities|FlowControl|DoOnce false :!label _label
      (:Completed
        (Utilities|IsValid Enemy :!label _label_2
          (:Is%20Valid
            (if (< (Transformation|GetDistanceTo Enemy self) (Variables|Default|GetHitRangex)) :!label _label_3
              (CallFunction|AIAttack)
              (Utilities|FlowControl|Delay (Math|Random|RandomFloatinRange 0.3 1.0))
              (if (Variables|Default|GetAttacking)
                (goto _label_2)
                (else
                  (goto _label Reset)))
              (else
                (AI|Navigation|SimpleMovetoLocation (Pawn|GetController self) (+ (* (Math|Vector|Normalize (- (Transformation|GetActorLocation) _returnvalue)) (* (Variables|Default|GetHitRangex) 0.6)) _returnvalue))
                (Utilities|FlowControl|Delay 2.0)
                (goto _label_3)))))))))

(fn ConstructionScript
  (|CallParentFunction))